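; BP_DiceRoller is the actor that runs a dice-rolling setup, spawning physical polyhedral dice with a chosen material and impulse direction.
; On BeginPlay it creates roll, amount and material widgets and enables mouse cursor and click events.
; Spawn, respawn-cocked, respawn-selected and per-tick checks are delegated to its BPACDiceRoller component.
; The construction script has that component build a configurable spawn grid, optionally previewed through an instanced static mesh.
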(event Custom|Spawn%20Dice
  ;[1 1 1] Spawn Selected Dice
  (Default|SpawnDice (Variables|Default|GetBPAC_DiceRoller) (Variables|SpawnDiceAmounts|GetD4Amount) (Variables|SpawnDiceAmounts|GetD6Amount) (Variables|SpawnDiceAmounts|GetD8Amount) (Variables|SpawnDiceAmounts|GetD10Amount) (Variables|SpawnDiceAmounts|GetD1000Amount) (Variables|SpawnDiceAmounts|GetD1010Amount) (Variables|SpawnDiceAmounts|GetD12Amount) (Variables|SpawnDiceAmounts|GetD20Amount) (Variables|SpawnDetails|GetDiceMaterial) (Variables|SpawnDetails|GetImpulse%20Direction) false))

(event Custom|ReSpawnCocked
  ;[1 1 1] Respawn Cocked Dice
  (Default|RespawnCocked (Variables|Default|GetBPAC_DiceRoller) (Variables|SpawnDetails|GetImpulse%20Direction) (Variables|SpawnDetails|GetDiceMaterial)))

(event Custom|Respawn%20Selected
  ;[1 1 1] ReSpawn Selected
  (Default|RespawnSelected (Variables|Default|GetBPAC_DiceRoller) (Variables|SpawnDetails|GetImpulse%20Direction) (Variables|SpawnDetails|GetDiceMaterial)))

(event EventBeginPlay
  (bind _returnvalue (Game|GetPlayerController 0))
  ;[1 1 1] Setup and Widget Components
  (bind _returnvalue_2 (UserInterface|CreateWidget "/Game/RandomsDiceRoller/UI/UI_DiceRoll.UI_DiceRoll_C"))
  (UserInterface|Viewport|AddtoViewport _returnvalue_2 0)
  (bind _returnvalue_3 (UserInterface|CreateWidget "/Game/RandomsDiceRoller/UI/UI_DiceAmounts.UI_DiceAmounts_C"))
  (UserInterface|Viewport|AddtoViewport _returnvalue_3 0)
  (bind _returnvalue_4 (UserInterface|CreateWidget "/Game/RandomsDiceRoller/UI/UI_MaterialChanger.UI_MaterialChanger_C"))
  (UserInterface|Viewport|AddtoViewport _returnvalue_4 0)
  (Input|EnableInput _returnvalue)
  (Variables|/Script/Engine.PlayerController|SetbShowMouseCursor _returnvalue true)
  (Variables|/Script/Engine.PlayerController|SetbEnableMouseOverEvents _returnvalue true)
  (Variables|/Script/Engine.PlayerController|SetbEnableClickEvents _returnvalue true))

(event EventTick
  (params (DeltaSeconds :type Float%20%28single-precision%29))
  ;[1 1 1] Tick Checks
  (Default|TickChecks (Variables|Default|GetBPAC_DiceRoller) false))

(fn ConstructionScript
  (Default|MakeGrid (Variables|Default|GetBPAC_DiceRoller) self (Variables|SpawnDetails|GetGrid%20X%20Spawns) (Variables|SpawnDetails|GetGrid%20Y%20Spawns) (Variables|SpawnDetails|GetGrid%20Z%20Spawns) (Variables|SpawnDetails|GetGrid%20Spacing) (Variables|SpawnDetails|GetGridShowSpawn) (Variables|Default|GetInstancedStaticMesh)))