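; Base dice actor that detects when it comes to rest and shows its result in a floating widget.
; BPACDice configures the die from a data table and checks the result once velocity reaches zero after a short delay, re-arming when it moves.
; The widget follows above the die facing the camera, showing the face value or a "C" cocked warning.
; Hover reveals valid results; clicking toggles selection and colours.
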(event OnBeginCursorOver(Dice)
  (params (TouchedComponent :type Primitive%20Component%20Object%20Reference))
  ;[1 1 1] Mouse Interactions
  (if (not (Variables|Default|GetIsSelected?))
    (Utilities|FaceValueNil
      (:false
        (Rendering|SetVisibility (Variables|Default|GetInfoWidget) true false)))))

(event OnEndCursorOver(Dice)
  (params (TouchedComponent :type Primitive%20Component%20Object%20Reference))
  ;[1 1 1] Mouse Interactions
  (if (not (Variables|Default|GetIsSelected?))
    (Utilities|FaceValueNil
      (:false
        (Rendering|SetVisibility (Variables|Default|GetInfoWidget) false false)))))

(event OnClicked(Dice)
  (params (TouchedComponent :type Primitive%20Component%20Object%20Reference) (ButtonPressed :type Key%20Structure :default "None"))
  ;[1 1 1] Mouse Interactions
  (Utilities|FaceValueNil
    (:false
      (if (Variables|Default|GetIsSelected?)
        (Variables|Default|SetIsSelected? false)
        (Rendering|SetVisibility (Variables|Default|GetInfoWidget) false false)
        (bind _asui_dice_local (Utilities|CasttoWidget))
        (Variables|/Game/RandomsDiceRoller/UI/UI_DiceLocal.UI_DiceLocal_C|SetText%20Colour _asui_dice_local (Variables|Default|GetWidget%20Text%20Colour%20Normal))
        (Variables|/Game/RandomsDiceRoller/UI/UI_DiceLocal.UI_DiceLocal_C|SetIcon%20Colour _asui_dice_local (Variables|Default|GetWidget%20Icon%20Colour%20Normal))
        (else
          (Variables|Default|SetIsSelected? true)
          (Rendering|SetVisibility (Variables|Default|GetInfoWidget) true false)
          (bind _asui_dice_local_2 (Utilities|CasttoWidget))
          (Variables|/Game/RandomsDiceRoller/UI/UI_DiceLocal.UI_DiceLocal_C|SetText%20Colour _asui_dice_local_2 (Variables|Default|GetWidget%20Text%20Colour%20Selected))
          (Variables|/Game/RandomsDiceRoller/UI/UI_DiceLocal.UI_DiceLocal_C|SetIcon%20Colour _asui_dice_local_2 (Variables|Default|GetWidget%20Icon%20Colour%20Selected)))))))

(event Custom|Destroy%20Self
  ;[1 1 1] Clear
  (Actor|DestroyActor))

(event Custom|ShowUIOff
  (Variables|Default|SetIsSelected? false)
  (Rendering|SetVisibility (Variables|Default|GetInfoWidget) false false)
  (bind _asui_dice_local (Utilities|CasttoWidget))
  (Variables|/Game/RandomsDiceRoller/UI/UI_DiceLocal.UI_DiceLocal_C|SetText%20Colour _asui_dice_local (Variables|Default|GetWidget%20Text%20Colour%20Normal))
  (Variables|/Game/RandomsDiceRoller/UI/UI_DiceLocal.UI_DiceLocal_C|SetIcon%20Colour _asui_dice_local (Variables|Default|GetWidget%20Icon%20Colour%20Normal)))

(event Custom|ShowUIOn
  (Variables|Default|SetIsSelected? true)
  (Rendering|SetVisibility (Variables|Default|GetInfoWidget) true false)
  (bind _asui_dice_local (Utilities|CasttoWidget))
  (Variables|/Game/RandomsDiceRoller/UI/UI_DiceLocal.UI_DiceLocal_C|SetText%20Colour _asui_dice_local (Variables|Default|GetWidget%20Text%20Colour%20Selected))
  (Variables|/Game/RandomsDiceRoller/UI/UI_DiceLocal.UI_DiceLocal_C|SetIcon%20Colour _asui_dice_local (Variables|Default|GetWidget%20Icon%20Colour%20Selected)))

(event EventBeginPlay
  ;[1 1 1] Setup
  (Default|SetStruct (Variables|Default|GetBPAC_Dice) (Variables|Default|GetDiceData) (Variables|Default|GetDataTableRow) (Variables|Default|GetDice))
  (bind _asui_dice_local (Utilities|CasttoWidget))
  (Variables|/Game/RandomsDiceRoller/UI/UI_DiceLocal.UI_DiceLocal_C|SetText%20Colour _asui_dice_local (Variables|Default|GetWidget%20Text%20Colour%20Normal))
  (Variables|/Game/RandomsDiceRoller/UI/UI_DiceLocal.UI_DiceLocal_C|SetIcon%20Colour _asui_dice_local (Variables|Default|GetWidget%20Icon%20Colour%20Normal)))

(event EventTick
  (params (DeltaSeconds :type Float%20%28single-precision%29))
  ;[1 1 1] Tick Checks
  (Utilities|WidgetTickSettings)
  (Utilities|FlowControl|Delay 0.2)
  (Utilities|DoOnceifStationary
    (:Stationary
      (Default|CheckResult (Variables|Default|GetBPAC_Dice) (Variables|Default|GetDice) (Variables|Default|GetDataTableRow))
      (Utilities|FaceValueNil
        (:True
          (Rendering|SetVisibility (Variables|Default|GetInfoWidget) true false))))))

(fn ConstructionScript)